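; Player character for in-game level editing, forwarding editor input to SKGLevelEditorHandler.
; On possession or remote BeginPlay it initializes the handler, and the local player gets the W_MapEditor widget, refreshed by handler change events.
; Hotkeys drive selection, placement, gizmos, clipboard and undo/redo, while axes and mouse wheel control SKGMLECharacterMovement flight and speed.
; Y or F returns to the previous pawn, and F or unpossession restores game-only input.
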(event `self.ReceivePossessed`
  (params (NewController :type "Controller Object Reference"))
  (bind _skgleveleditorhandler (`self.SKGLevelEditorHandler`))
  (`SKGMLEHandlerComponent.Init` (`self.SKGLevelEditorHandler`) :!label _label)
  (if (`self.IsLocallyControlled`)
    (`self.HandleHUD`)
    (add `SKGMLEHandlerComponent.OnHistoryChangedDelegate` _skgleveleditorhandler (delegate `OnHistoryChanged`))
    (add `SKGMLEHandlerComponent.OnChangeDelegate` _skgleveleditorhandler (delegate `OnChange`))))

(event `self.ReceiveBeginPlay`
  (`/Engine/EditorBlueprintResources/ActorMacros.Switch Has Authority`
    (:`Remote`
      (goto _label))))

(event `OnChange`
  (params (ActionType :type "ESKGMLEActionType Enum" :default "Grab"))
  (`/Game/LevelEditor/UI/W_MapEditor.UpdateUI` (`self.W_MapEditor`) ActionType))

(event `OnHistoryChanged`
  (params (ActionType :type "ESKGMLEHistoryActionType Enum" :default "Undo")))

(event `Key|Ctrl+Z`
  (params (Key :type "Key Structure"))
  (:`Pressed`
    (`SKGMLEHandlerComponent.Undo` (`self.SKGLevelEditorHandler`))))

(event `InputAxis|MoveForward`
  (params (AxisValue :type "Float (single-precision)"))
  (bind _asskgmlecharacter_movement (cast `SKGMLECharacterMovement` (`self.CharacterMovement`)))
  (`SKGMLECharacterMovement.MoveForward` _asskgmlecharacter_movement AxisValue))

(event `Key|Ctrl+Y`
  (params (Key :type "Key Structure"))
  (:`Pressed`
    (`SKGMLEHandlerComponent.Redo` (`self.SKGLevelEditorHandler`))))

(event `InputAxis|MoveRight`
  (params (AxisValue :type "Float (single-precision)"))
  (bind _asskgmlecharacter_movement (cast `SKGMLECharacterMovement` (`self.CharacterMovement`)))
  (`SKGMLECharacterMovement.MoveRight` _asskgmlecharacter_movement AxisValue))

(event `InputAxis|MoveUp`
  (params (AxisValue :type "Float (single-precision)"))
  (bind _asskgmlecharacter_movement (cast `SKGMLECharacterMovement` (`self.CharacterMovement`)))
  (`SKGMLECharacterMovement.MoveUp` _asskgmlecharacter_movement AxisValue))

(event `Key|Y`
  (params (Key :type "Key Structure"))
  (:`Pressed`
    (`SKGMLEHandlerComponent.EnterMovementMode` (`self.SKGLevelEditorHandler`) true)
    (`Widget.RemoveFromParent` (`self.W_MapEditor`))
    (`SKGMLEHandlerComponent.UnpossessToReturnPawn` (`self.SKGLevelEditorHandler`))))

(event `InputAxis|Turn`
  (params (AxisValue :type "Float (single-precision)"))
  (bind _asskgmlecharacter_movement (cast `SKGMLECharacterMovement` (`self.CharacterMovement`)))
  (`SKGMLECharacterMovement.Turn` _asskgmlecharacter_movement AxisValue))

(event `InputAxis|LookUp`
  (params (AxisValue :type "Float (single-precision)"))
  (bind _asskgmlecharacter_movement (cast `SKGMLECharacterMovement` (`self.CharacterMovement`)))
  (`SKGMLECharacterMovement.LookUp` _asskgmlecharacter_movement AxisValue))

(event `Key|Ctrl+C`
  (params (Key :type "Key Structure"))
  (:`Pressed`
    (`SKGMLEHandlerComponent.CopySelection` (`self.SKGLevelEditorHandler`))))

(event `Key|F`
  (params (Key :type "Key Structure"))
  ;[0 1 0] Example of going back to return pawn
  (:`Pressed`
    (`self.OnUnpossess`)
    (`SKGMLEHandlerComponent.UnpossessToReturnPawn` (`self.SKGLevelEditorHandler`))))

(event `Key|Ctrl+V`
  (params (Key :type "Key Structure"))
  (:`Pressed`
    (`SKGMLEHandlerComponent.Paste` (`self.SKGLevelEditorHandler`) true)))

(event `Key|RightMouseButton`
  (params (Key :type "Key Structure"))
  (bind _skgleveleditorhandler (`self.SKGLevelEditorHandler`))
  (:`Pressed`
    (`SKGMLEHandlerComponent.EnterMovementMode` _skgleveleditorhandler true))
  (:`Released`
    (`SKGMLEHandlerComponent.EnterMovementMode` _skgleveleditorhandler false)))

(event `OnUnpossess`
  (bind _returnvalue (`GameplayStatics.GetPlayerController` 0))
  ;[0 1 0] Example of going back to return pawn
  (if (`self.IsLocallyControlled`) :!label _label_2
    (`Widget.RemoveFromParent` (`self.W_MapEditor`))
    (`WidgetBlueprintLibrary.SetInputMode_GameOnly` _returnvalue)
    (set `PlayerController.bShowMouseCursor` false _returnvalue)))

(event `self.ReceiveUnpossessed`
  (params (OldController :type "Controller Object Reference"))
  ;[0 1 0] Example of going back to return pawn
  (goto _label_2))

(event `Key|Delete`
  (params (Key :type "Key Structure"))
  (:`Pressed`
    (`SKGMLEHandlerComponent.DeleteSelection` (`self.SKGLevelEditorHandler`) false)))

(event `Key|Alt+LeftMouseButton`
  (params (Key :type "Key Structure"))
  (:`Pressed`
    (`SKGMLEHandlerComponent.TryDuplicateDrag` (`self.SKGLevelEditorHandler`))))

(event `Key|LeftMouseButton`
  (params (Key :type "Key Structure"))
  (bind _skgleveleditorhandler (`self.SKGLevelEditorHandler`))
  (:`Pressed`
    (if (`SKGMLEHandlerComponent.IsDraggingLocalActor` _skgleveleditorhandler)
      (`SKGMLEHandlerComponent.PlacePrePlacedActor` _skgleveleditorhandler)
      (else
        (`SKGMLEHandlerComponent.FindAndGrab` _skgleveleditorhandler false))))
  (:`Released`
    (`SKGMLEHandlerComponent.Release` _skgleveleditorhandler)))

(event `Key|MouseScrollUp`
  (params (Key :type "Key Structure"))
  (:`Pressed`
    (bind _asskgmlecharacter_movement (cast `SKGMLECharacterMovement` (`self.CharacterMovement`)))
    (`SKGMLECharacterMovement.IncreaseSpeedMultiplier` _asskgmlecharacter_movement 0.2)))

(event `Key|Shift+LeftMouseButton`
  (params (Key :type "Key Structure"))
  (bind _skgleveleditorhandler (`self.SKGLevelEditorHandler`))
  (:`Pressed`
    (`SKGMLEHandlerComponent.FindAndGrab` _skgleveleditorhandler true))
  (:`Released`
    (`SKGMLEHandlerComponent.Release` _skgleveleditorhandler)))

(event `Key|MouseScrollDown`
  (params (Key :type "Key Structure"))
  (:`Pressed`
    (bind _asskgmlecharacter_movement (cast `SKGMLECharacterMovement` (`self.CharacterMovement`)))
    (`SKGMLECharacterMovement.DecreaseSpeedMultiplier` _asskgmlecharacter_movement 0.2)))

(event `Key|Z`
  (params (Key :type "Key Structure"))
  (bind _skgleveleditorhandler (`self.SKGLevelEditorHandler`))
  (:`Pressed`
    (`/Engine/EditorBlueprintResources/StandardMacros.FlipFlop`
      (:`A`
        (`SKGMLEHandlerComponent.SetCoordinateSystem` _skgleveleditorhandler "World"))
      (:`B`
        (`SKGMLEHandlerComponent.SetCoordinateSystem` _skgleveleditorhandler "Relative")))))

(event `Key|X`
  (params (Key :type "Key Structure"))
  (bind _skgleveleditorhandler (`self.SKGLevelEditorHandler`))
  (:`Pressed`
    (`/Engine/EditorBlueprintResources/StandardMacros.FlipFlop`
      (:`A`
        (`SKGMLEHandlerComponent.EnableHighlightingOfSelection` _skgleveleditorhandler false))
      (:`B`
        (`SKGMLEHandlerComponent.EnableHighlightingOfSelection` _skgleveleditorhandler true)))))

(event `Key|Q`
  (params (Key :type "Key Structure"))
  (:`Pressed`
    (`SKGMLEHandlerComponent.SetGizmoType` (`self.SKGLevelEditorHandler`) "All")))

(event `Key|W`
  (params (Key :type "Key Structure"))
  (:`Pressed`
    (`SKGMLEHandlerComponent.SetGizmoType` (`self.SKGLevelEditorHandler`) "Translation")))

(event `Key|E`
  (params (Key :type "Key Structure"))
  (:`Pressed`
    (`SKGMLEHandlerComponent.SetGizmoType` (`self.SKGLevelEditorHandler`) "Rotation")))

(event `Key|R`
  (params (Key :type "Key Structure"))
  (:`Pressed`
    (`SKGMLEHandlerComponent.SetGizmoType` (`self.SKGLevelEditorHandler`) "Scale")))

(fn `HandleHUD`
  (bind _w_mapeditor (`self.W_MapEditor`))
  (if (`self.IsLocallyControlled`)
    (`/Engine/EditorBlueprintResources/StandardMacros.IsValid` _w_mapeditor
      (:`Is Valid`
        (if (not (`Widget.IsInViewport` _w_mapeditor))
          (`UserWidget.AddToViewport` (`self.W_MapEditor`) 0)
          (`WidgetBlueprintLibrary.SetInputMode_GameAndUIEx` (`GameplayStatics.GetPlayerController` 0) (`self.W_MapEditor`) "DoNotLock" false :!label _label)))
      (:`Is Not Valid`
        (bind _returnvalue (`|CreateWidget` "/Game/LevelEditor/UI/W_MapEditor.W_MapEditor_C" null (`self.SKGLevelEditorHandler`)))
        (bind _output_get (set `self.W_MapEditor` _returnvalue))
        (`UserWidget.AddToViewport` _output_get 0)
        (goto _label)))))

(fn `UserConstructionScript`)